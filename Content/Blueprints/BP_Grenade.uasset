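; BP_Grenade is a grenade actor that explodes on a short fuse or when it hits something damageable.
; A timer started on BeginPlay and the Hit event both call Explode.
; Explode spawns an explosion emitter, applies radial damage with falloff credited to the instigator controller, draws a debug sphere at the outer radius, then destroys the actor.
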(event `self.ReceiveBeginPlay`
  (`KismetSystemLibrary.K2_SetTimerDelegate` (delegate `Explode`) 1.0))

(event `Explode`
  (bind _returnvalue (`self.K2_GetActorLocation`))
  (`GameplayStatics.SpawnEmitterAtLocation` "/Game/WeaponEffects/Explosion/P_Explosion.P_Explosion" _returnvalue)
  (`GameplayStatics.ApplyRadialDamageWithFalloff` :`BaseDamage` (`self.DamageAmount`) :`Origin` _returnvalue :`DamageInnerRadius` (`self.DamageInnerRadius`) :`DamageOuterRadius` (`self.DamageOuterRadius`) :`DamageFalloff` 1.0 :`DamageCauser` self :`InstigatedByController` (`self.GetInstigatorController`))
  (`KismetSystemLibrary.DrawDebugSphere` _returnvalue (`self.DamageOuterRadius`) 12 (struct :`R` 1.0 :`G` 0.862932 :`B` 0.028789 :`A` 1.0) 1.0 2.0)
  (`self.K2_DestroyActor`))

(event `self.ReceiveHit`
  (params (MyComp :type "PrimitiveComponent Object Reference") (Other :type "Actor Object Reference") (OtherComp :type "PrimitiveComponent Object Reference") (bSelfMoved :type Boolean) (HitLocation :type "Vector Structure") (HitNormal :type "Vector Structure") (NormalImpulse :type "Vector Structure") (Hit :type "HitResult Structure (by ref)"))
  (if (`Actor.bCanBeDamaged` Other)
    (`self.Explode`)))

(fn `UserConstructionScript`)